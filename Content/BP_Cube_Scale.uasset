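; BP_Cube_Scale is an actor, named as a cube, that shrinks each time another actor begins overlapping it.
; At BeginPlay it stores a scale step equal to its starting scale times the Procent variable.
; Each overlap subtracts that fixed step, so shrinking is linear, with no filter on the other actor and no lower limit.
; The overlap also applies a zero world offset, which leaves the position unchanged.
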(event EventBeginPlay
  (|CallParentFunction)
  (Variables|Default|SetDeltaScale (* (Transformation|GetActorScale3D) (Variables|Default|GetProcent))))

(event Collision|EventActorBeginOverlap
  (params (OtherActor :type Actor%20Object%20Reference))
  (|CallParentFunction OtherActor)
  (Transformation|AddActorWorldOffset "0, 0, 0")
  (Transformation|SetActorScale3D (- (Transformation|GetActorScale3D) (Variables|Default|GetDeltaScale))))

(event EventTick
  (params (DeltaSeconds :type Float%20%28single-precision%29))
  (|CallParentFunction DeltaSeconds) ; This node is disabled and will not be called.\nDrag off pins to build functionality.
)

(fn ConstructionScript
  (|CallParentFunction))