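; BP_Cube_Material is an actor Blueprint that changes the material of its Cube when another actor begins overlapping it.
; The overlap event calls the parent handler, applies a zero world offset that leaves the actor in place, then sets BP_Material on the first material slot if Cube is valid.
; BeginPlay and Tick are disabled, and the construction script only calls its parent.
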(event EventBeginPlay
  (|CallParentFunction) ; This node is disabled and will not be called.\nDrag off pins to build functionality.
)

(event Collision|EventActorBeginOverlap
  (params (OtherActor :type Actor%20Object%20Reference))
  (|CallParentFunction OtherActor)
  (Transformation|AddActorWorldOffset "0, 0, 0")
  (Utilities|IsValid (Variables|Default|GetCube)
    (:Is%20Valid
      (Rendering|Material|SetMaterial (Variables|Default|GetCube) 0 "/Game/BP_Material.BP_Material"))))

(event EventTick
  (params (DeltaSeconds :type Float%20%28single-precision%29))
  (|CallParentFunction DeltaSeconds) ; This node is disabled and will not be called.\nDrag off pins to build functionality.
)

(fn ConstructionScript
  (|CallParentFunction))